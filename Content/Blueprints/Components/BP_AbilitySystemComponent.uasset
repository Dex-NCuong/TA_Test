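; Custom ability component that spawns and activates a BP_ThirdPersonCharacter owner's abilities by slot index.
; ActivateAbility spawns the indexed ability actor at the owner, passes it its data and character, then activates it if CanActivate passes or destroys it otherwise.
; Successful activation starts a hardcoded timer cooldown for the first three slots, with per-slot ready flags that ActivateAbility itself never checks.
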(event EventBeginPlay)

(event EventTick
  (params (DeltaSeconds :type Float%20%28single-precision%29)))

(fn ActivateAbility
  (params (Index :type Integer))
  (bind _self self)
  (bind _returnvalue (Components|GetOwner _self))
  (if (Utilities|Array|IsValidIndex (Variables|Default|GetAbilities) Index)
    (bind _returnvalue_2 (Game|SpawnActorfromClass (Utilities|Array|Get(acopy) (Variables|Default|GetAbilities) Index) (Math|Transform|MakeTransform (Transformation|GetActorLocation _returnvalue)) "AlwaysSpawn" "MultiplyWithRoot" _returnvalue 0))
    (bind _asbp_ability_base (Utilities|Casting|CastToBP_AbilityBase _returnvalue_2))
    (Variables|/Game/Blueprints/Ability/BP_AbilityBase.BP_AbilityBase_C|SetAbilityData _asbp_ability_base (Utilities|Array|Get(acopy) (Variables|Default|GetAbilityDataList) Index))
    (bind _asbp_third_person_character (Utilities|Casting|CastToBP_ThirdPersonCharacter _returnvalue)
      (:then
        (Variables|/Game/Blueprints/Ability/BP_AbilityBase.BP_AbilityBase_C|SetOwnerCharacter _asbp_ability_base _asbp_third_person_character)
        (bind _returnvalue_3 (Default|CanActivate _asbp_ability_base))
        (if _returnvalue_3
          (Default|Activate _asbp_ability_base)
          (CallFunction|StartCooldown Index)
          (else
            (Actor|DestroyActor _asbp_ability_base))))
      (:CastFailed
        (Actor|DestroyActor _asbp_ability_base)))))

(fn CooldownFinished0
  (Variables|Default|SetAbility0Ready true))

(fn CooldownFinished1
  (Variables|Default|SetAbility1Ready true))

(fn CooldownFinished2
  (Variables|Default|SetAbility2Ready true))

(fn StartCooldown
  (params (Index :type Integer))
  (switch int Index
    (:0
      (Variables|Default|SetAbility0Ready false)
      (Utilities|Time|SetTimerbyEvent (EventDispatchers|CreateEvent :!event CooldownFinished0) 3.0))
    (:1
      (Variables|Default|SetAbility1Ready false)
      (Utilities|Time|SetTimerbyEvent (EventDispatchers|CreateEvent :!event CooldownFinished1) 5.0))
    (:2
      (Variables|Default|SetAbility2Ready false)
      (Utilities|Time|SetTimerbyEvent (EventDispatchers|CreateEvent :!event CooldownFinished2) 4.0))))