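; Heal ability actor that restores a fixed amount of health to its owning character.
; On Activate it prints a debug message, adds the flat heal to OwnerCharacter's Health clamped between zero and MaxHealth, then immediately calls EndAbility.
; BeginPlay, overlap, Tick and construction only forward to the parent class.
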(event EventBeginPlay
  (|CallParentFunction))

(event Collision|EventActorBeginOverlap
  (params (OtherActor :type Actor%20Object%20Reference))
  (|CallParentFunction OtherActor))

(event EventTick
  (params (DeltaSeconds :type Float%20%28single-precision%29))
  (|CallParentFunction DeltaSeconds))

(event EventActivate
  (bind _ownercharacter (Variables|Default|GetOwnerCharacter))
  (Development|PrintString "Heal: Increase Health")
  (Variables|/Game/ThirdPerson/Blueprints/BP_ThirdPersonCharacter.BP_ThirdPersonCharacter_C|SetHealth _ownercharacter (Math|Float|Clamp(Float) (+ (Variables|/Game/ThirdPerson/Blueprints/BP_ThirdPersonCharacter.BP_ThirdPersonCharacter_C|GetHealth _ownercharacter) (Math|Float|MakeLiteralFloat 3e+01)) 0.0 (Variables|/Game/ThirdPerson/Blueprints/BP_ThirdPersonCharacter.BP_ThirdPersonCharacter_C|GetMaxHealth _ownercharacter)))
  (CallFunction|EndAbility))

(fn ConstructionScript
  (|CallParentFunction))