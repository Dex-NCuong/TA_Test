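; Fireball ability that plays its cast montage and launches a projectile from the owning character.
; Activation ignores move input while the montage plays, then restores it and ends the ability on completion or interruption.
; The montage's Cast notify plays a fire sound and spawns BP_FireballProjectile ahead of the character, passing it the damage from AbilityData.
; The sound and projectile only fire when the owner has a PlayerController.
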(event Custom|ReceiveBeginPlay_2)

(event Custom|ReceiveActorBeginOverlap_2
  (params (OtherActor :type Actor%20Object%20Reference)))

(event EventActivate
  (bind _self self)
  (bind _ownercharacter (Variables|Default|GetOwnerCharacter))
  (bind _abilitydata (Variables|Default|GetAbilityData))
  (bind _returnvalue (Pawn|GetController _ownercharacter))
  (bind _returnvalue_2 (Transformation|GetActorLocation _ownercharacter))
  (Input|SetIgnoreMoveInput _returnvalue true)
  (bind _notifyname (Animation|Montage|PlayMontage (Variables|/Script/Engine.Character|GetMesh _ownercharacter) (Variables|/Game/Blueprints/Data/DA_AbilityData.DA_AbilityData_C|GetAnimation _abilitydata))
    (:OnCompleted
      (Input|SetIgnoreMoveInput _returnvalue false :!label _label)
      (CallFunction|EndAbility))
    (:OnInterrupted
      (goto _label))
    (:OnNotifyBegin
      (if (== _notifyname "Cast")
        (Utilities|Casting|CastToPlayerController (Pawn|GetController _ownercharacter))
        (Audio|PlaySoundatLocation _self "/Game/Blueprints/Sound/FireSound.FireSound" _returnvalue_2 "0, 0, 0" 1.0 1.0 0.0 0 0 0 0)
        (bind _returnvalue_3 (Game|SpawnActorfromClass _self "/Game/Blueprints/Ability/BP_FireballProjectile.BP_FireballProjectile_C" (Math|Transform|MakeTransform (+ _returnvalue_2 (* (Transformation|GetActorForwardVector _ownercharacter) (Math|Float|MakeLiteralFloat 1.5e+02))) (Transformation|GetActorRotation _ownercharacter)) "AlwaysSpawn" "MultiplyWithRoot" _ownercharacter 0))
        (Variables|/Game/Blueprints/Ability/BP_FireballProjectile.BP_FireballProjectile_C|SetDamage _returnvalue_3 (Variables|/Game/Blueprints/Data/DA_AbilityData.DA_AbilityData_C|GetDamage _abilitydata))))))

(fn ConstructionScript
  (|CallParentFunction))