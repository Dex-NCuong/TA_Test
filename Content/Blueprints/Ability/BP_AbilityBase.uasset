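; Base ability Blueprint that plays an animation montage on its owning character, with costs and animation read from AbilityData.
; CanActivate checks cooldown, mana and stamina, but Execute calls Activate without that check.
; EndAbility deducts mana and clears the cooldown flag, as does ResetCooldown for the flag.
; Nothing here sets the cooldown, and the stamina deduction is left unconnected.
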(fn ConstructionScript)

(fn CanActivate
  (bind _abilitydata (Variables|Default|GetAbilityData))
  (bind _ownercharacter (Variables|Default|GetOwnerCharacter))
  (if (Variables|Default|GetIsOnCooldown)
    (return false)
    (else
      (if (< (Variables|/Game/ThirdPerson/Blueprints/BP_ThirdPersonCharacter.BP_ThirdPersonCharacter_C|GetMana _ownercharacter) (Variables|/Game/Blueprints/Data/DA_AbilityData.DA_AbilityData_C|GetManaCost _abilitydata))
        _
        (elif (< (Variables|/Game/ThirdPerson/Blueprints/BP_ThirdPersonCharacter.BP_ThirdPersonCharacter_C|GetStamina _ownercharacter) (Variables|/Game/Blueprints/Data/DA_AbilityData.DA_AbilityData_C|GetStaminaCost _abilitydata))
          _
          (else
            (return true))))
      (return false))))

(fn Activate
  (Animation|Montage|MontagePlay (Components|SkeletalMesh|GetAnimInstance (Variables|/Script/Engine.Character|GetMesh (Variables|Default|GetOwnerCharacter))) (Variables|/Game/Blueprints/Data/DA_AbilityData.DA_AbilityData_C|GetAnimation (Variables|Default|GetAbilityData)) 1.0 "MontageLength" 0.0 true))

(fn EndAbility
  (bind _ownercharacter (Variables|Default|GetOwnerCharacter))
  (Variables|/Game/ThirdPerson/Blueprints/BP_ThirdPersonCharacter.BP_ThirdPersonCharacter_C|SetMana _ownercharacter (- (Variables|/Game/ThirdPerson/Blueprints/BP_ThirdPersonCharacter.BP_ThirdPersonCharacter_C|GetMana _ownercharacter) (Variables|/Game/Blueprints/Data/DA_AbilityData.DA_AbilityData_C|GetManaCost (Variables|Default|GetAbilityData))))
  (Variables|Default|SetIsOnCooldown false))

(fn ResetCooldown
  (Variables|Default|SetIsOnCooldown false))

(fn Execute
  (CallFunction|Activate))