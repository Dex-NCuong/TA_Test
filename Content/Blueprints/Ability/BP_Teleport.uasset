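; BP_Teleport is an ability that blinks its owner character 600 units along its forward vector when activated.
; It plays a teleport sound at the owner's location, then line traces on the Visibility channel to find obstacles.
; On a blocking hit it stops 50 units short of the impact point; otherwise it moves the full distance with a swept teleport, then ends the ability.
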(event Custom|ReceiveBeginPlay_2)

(event Custom|ReceiveActorBeginOverlap_2
  (params (OtherActor :type Actor%20Object%20Reference)))

(event EventActivate
  (bind _returnvalue (Math|Float|MakeLiteralFloat 6e+02))
  (bind _ownercharacter (Variables|Default|GetOwnerCharacter))
  (bind _ownercharacter_2 (Variables|Default|GetOwnerCharacter))
  (bind _returnvalue_2 (Transformation|GetActorLocation _ownercharacter))
  (bind _returnvalue_3 (Transformation|GetActorForwardVector _ownercharacter_2))
  (bind _returnvalue_4 (* _returnvalue_3 _returnvalue))
  (bind _returnvalue_5 (+ _returnvalue_2 _returnvalue_4))
  ;[0.15 0.15 0.15 0.5] TelePort 600m
  (Audio|PlaySoundatLocation _ownercharacter "/Game/Blueprints/Sound/TelePortSound.TelePortSound" (Transformation|GetActorLocation _ownercharacter) "0, 0, 0" 1.0 1.0 0.0 0 0 0 0)
  (Utilities|IsValid _ownercharacter
    (:Is%20Valid
      (bind _outhit (Collision|LineTraceByChannel _ownercharacter _returnvalue_2 _returnvalue_5 "TraceTypeQuery1" false 0 "None"))
      (if (.bBlockingHit (Collision|BreakHitResult _outhit))
        (Transformation|SetActorLocation (Variables|Default|GetOwnerCharacter) (- (.ImpactPoint (Collision|BreakHitResult _outhit)) (* _returnvalue_3 (Math|Float|MakeLiteralFloat 5e+01))) true true)
        (else
          (Transformation|SetActorLocation (Variables|Default|GetOwnerCharacter) _returnvalue_5 true true)))
      (CallFunction|EndAbility))
    (:Is%20Not%20Valid
      (CallFunction|EndAbility))))

(fn ConstructionScript
  (|CallParentFunction))