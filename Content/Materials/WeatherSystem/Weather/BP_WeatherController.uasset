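; Weather controller that drives global wetness, snow, temperature and time-of-day sun and sky colors through the MPC_GlobalWeather material parameter collection.
; Preview events set weather presets or jump the clock, and ApplyWeatherImmediate snaps straight to the targets.
; Tick eases weather from old to target values with a smoothstep over TransitionDuration and, when enabled, advances a 24-hour clock blending four color keyframes.
; Older FInterpTo and sine-based graphs remain disconnected, and both color helper functions are empty.
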(event Custom|PreviewDry
  (Variables|Transition|SetOldWetness (Variables|RuntimeState|GetCurrentWetness))
  (Variables|Transition|SetOldSnow (Variables|RuntimeState|GetCurrentSnow))
  (Variables|Transition|SetOldTemperature (Variables|RuntimeState|GetCurrentTemperatureC))
  (Variables|WeatherTargets|SetWetnessTarget 0.0)
  (Variables|WeatherTargets|SetSnowTarget 0.0)
  (Variables|WeatherTargets|SetTemperatureTargetC 22.0)
  (Variables|Transition|SetTransitionProgress 0.0)
  (Variables|Transition|SetIsTransitioning true))

(event Custom|PreviewRain
  (Variables|Transition|SetOldWetness (Variables|RuntimeState|GetCurrentWetness))
  (Variables|Transition|SetOldSnow (Variables|RuntimeState|GetCurrentSnow))
  (Variables|Transition|SetOldTemperature (Variables|RuntimeState|GetCurrentTemperatureC))
  (Variables|WeatherTargets|SetWetnessTarget 1.0)
  (Variables|WeatherTargets|SetSnowTarget 0.0)
  (Variables|WeatherTargets|SetTemperatureTargetC 8.0)
  (Variables|Transition|SetTransitionProgress 0.0)
  (Variables|Transition|SetIsTransitioning true))

(event Custom|PreviewSnow
  (Variables|Transition|SetOldWetness (Variables|RuntimeState|GetCurrentWetness))
  (Variables|Transition|SetOldSnow (Variables|RuntimeState|GetCurrentSnow))
  (Variables|Transition|SetOldTemperature (Variables|RuntimeState|GetCurrentTemperatureC))
  (Variables|WeatherTargets|SetWetnessTarget 0.25)
  (Variables|WeatherTargets|SetSnowTarget 1.0)
  (Variables|WeatherTargets|SetTemperatureTargetC -5.0)
  (Variables|Transition|SetTransitionProgress 0.0)
  (Variables|Transition|SetIsTransitioning true))

(event Custom|PreviewFrozen
  (Variables|Transition|SetOldWetness (Variables|RuntimeState|GetCurrentWetness))
  (Variables|Transition|SetOldSnow (Variables|RuntimeState|GetCurrentSnow))
  (Variables|Transition|SetOldTemperature (Variables|RuntimeState|GetCurrentTemperatureC))
  (Variables|WeatherTargets|SetWetnessTarget 0.65)
  (Variables|WeatherTargets|SetSnowTarget 0.35)
  (Variables|WeatherTargets|SetTemperatureTargetC -12.0)
  (Variables|Transition|SetTransitionProgress 0.0)
  (Variables|Transition|SetIsTransitioning true))

(event Custom|ApplyWeatherImmediate
  (bind _wetnesstarget (Variables|WeatherTargets|GetWetnessTarget))
  (bind _snowtarget (Variables|WeatherTargets|GetSnowTarget))
  (bind _temperaturetargetc (Variables|WeatherTargets|GetTemperatureTargetC))
  (Variables|RuntimeState|SetCurrentWetness _wetnesstarget)
  (Variables|RuntimeState|SetCurrentSnow _snowtarget)
  (Variables|RuntimeState|SetCurrentTemperatureC _temperaturetargetc)
  (Rendering|Material|SetScalarParameterValue "/Game/Materials/ParameterCollections/MPC_GlobalWeather.MPC_GlobalWeather" "WetnessAmount" _wetnesstarget :!class /Script/Engine.KismetMaterialLibrary)
  (Rendering|Material|SetScalarParameterValue "/Game/Materials/ParameterCollections/MPC_GlobalWeather.MPC_GlobalWeather" "SnowAmount" _snowtarget :!class /Script/Engine.KismetMaterialLibrary)
  (Rendering|Material|SetScalarParameterValue "/Game/Materials/ParameterCollections/MPC_GlobalWeather.MPC_GlobalWeather" "Temperature" _temperaturetargetc :!class /Script/Engine.KismetMaterialLibrary)
  (Variables|Transition|SetOldWetness _wetnesstarget)
  (Variables|Transition|SetOldSnow _snowtarget)
  (Variables|Transition|SetOldTemperature _temperaturetargetc)
  (Variables|Transition|SetTransitionProgress 1.0)
  (Variables|Transition|SetIsTransitioning false))

(event Custom|PreviewDawn
  (Variables|TimeOfDay|SetTimeOfDayHours 6.0)
  (Variables|TimeOfDay|SetEnableTimeOfDay true))

(event Custom|PreviewNoon
  (Variables|TimeOfDay|SetTimeOfDayHours 12.0)
  (Variables|TimeOfDay|SetEnableTimeOfDay true))

(event Custom|PreviewDusk
  (Variables|TimeOfDay|SetTimeOfDayHours 18.0)
  (Variables|TimeOfDay|SetEnableTimeOfDay true))

(event Custom|PreviewNight
  (Variables|TimeOfDay|SetTimeOfDayHours 0.0)
  (Variables|TimeOfDay|SetEnableTimeOfDay true))

(event EventBeginPlay
  (bind _wetnesstarget (Variables|WeatherTargets|GetWetnessTarget))
  (bind _snowtarget (Variables|WeatherTargets|GetSnowTarget))
  (bind _temperaturetargetc (Variables|WeatherTargets|GetTemperatureTargetC))
  (Variables|RuntimeState|SetCurrentWetness _wetnesstarget)
  (Variables|RuntimeState|SetCurrentSnow _snowtarget)
  (Variables|RuntimeState|SetCurrentTemperatureC _temperaturetargetc)
  (Variables|Transition|SetIsTransitioning false)
  (Variables|Transition|SetTransitionProgress 1.0)
  (Rendering|Material|SetScalarParameterValue "/Game/Materials/ParameterCollections/MPC_GlobalWeather.MPC_GlobalWeather" "WetnessAmount" _wetnesstarget :!class /Script/Engine.KismetMaterialLibrary)
  (Rendering|Material|SetScalarParameterValue "/Game/Materials/ParameterCollections/MPC_GlobalWeather.MPC_GlobalWeather" "SnowAmount" _snowtarget :!class /Script/Engine.KismetMaterialLibrary)
  (Rendering|Material|SetScalarParameterValue "/Game/Materials/ParameterCollections/MPC_GlobalWeather.MPC_GlobalWeather" "Temperature" _temperaturetargetc :!class /Script/Engine.KismetMaterialLibrary))

(event EventTick
  (params (DeltaSeconds :type Float%20%28single-precision%29))
  (Variables|Transition|SetTransitionProgress (Math|Float|Clamp(Float) (+ (Variables|Transition|GetTransitionProgress) (/ DeltaSeconds (Variables|Transition|GetTransitionDuration)))))
  (if (>= (Math|Float|Clamp(Float) (+ (Variables|Transition|GetTransitionProgress) (/ DeltaSeconds (Variables|Transition|GetTransitionDuration)))) (Math|Float|MakeLiteralFloat 1.0))
    (Variables|Transition|SetIsTransitioning false))
  (Variables|RuntimeState|SetCurrentWetness (Math|Float|Lerp (Variables|Transition|GetOldWetness) (Variables|WeatherTargets|GetWetnessTarget) (select (Variables|Transition|GetIsTransitioning) (* (* (Math|Float|Clamp(Float) (+ (Variables|Transition|GetTransitionProgress) (/ DeltaSeconds (Variables|Transition|GetTransitionDuration)))) (Math|Float|Clamp(Float) (+ (Variables|Transition|GetTransitionProgress) (/ DeltaSeconds (Variables|Transition|GetTransitionDuration))))) (- (Math|Float|MakeLiteralFloat 3.0) (* (Math|Float|MakeLiteralFloat 2.0) (Math|Float|Clamp(Float) (+ (Variables|Transition|GetTransitionProgress) (/ DeltaSeconds (Variables|Transition|GetTransitionDuration))))))) (Math|Float|MakeLiteralFloat 1.0))))
  (Variables|RuntimeState|SetCurrentSnow (Math|Float|Lerp (Variables|Transition|GetOldSnow) (Variables|WeatherTargets|GetSnowTarget) (select (Variables|Transition|GetIsTransitioning) (* (* (Math|Float|Clamp(Float) (+ (Variables|Transition|GetTransitionProgress) (/ DeltaSeconds (Variables|Transition|GetTransitionDuration)))) (Math|Float|Clamp(Float) (+ (Variables|Transition|GetTransitionProgress) (/ DeltaSeconds (Variables|Transition|GetTransitionDuration))))) (- (Math|Float|MakeLiteralFloat 3.0) (* (Math|Float|MakeLiteralFloat 2.0) (Math|Float|Clamp(Float) (+ (Variables|Transition|GetTransitionProgress) (/ DeltaSeconds (Variables|Transition|GetTransitionDuration))))))) (Math|Float|MakeLiteralFloat 1.0))))
  (Variables|RuntimeState|SetCurrentTemperatureC (Math|Float|Lerp (Variables|Transition|GetOldTemperature) (Variables|WeatherTargets|GetTemperatureTargetC) (select (Variables|Transition|GetIsTransitioning) (* (* (Math|Float|Clamp(Float) (+ (Variables|Transition|GetTransitionProgress) (/ DeltaSeconds (Variables|Transition|GetTransitionDuration)))) (Math|Float|Clamp(Float) (+ (Variables|Transition|GetTransitionProgress) (/ DeltaSeconds (Variables|Transition|GetTransitionDuration))))) (- (Math|Float|MakeLiteralFloat 3.0) (* (Math|Float|MakeLiteralFloat 2.0) (Math|Float|Clamp(Float) (+ (Variables|Transition|GetTransitionProgress) (/ DeltaSeconds (Variables|Transition|GetTransitionDuration))))))) (Math|Float|MakeLiteralFloat 1.0))))
  (Rendering|Material|SetScalarParameterValue "/Game/Materials/ParameterCollections/MPC_GlobalWeather.MPC_GlobalWeather" "WetnessAmount" (Math|Float|Lerp (Variables|Transition|GetOldWetness) (Variables|WeatherTargets|GetWetnessTarget) (select (Variables|Transition|GetIsTransitioning) (* (* (Math|Float|Clamp(Float) (+ (Variables|Transition|GetTransitionProgress) (/ DeltaSeconds (Variables|Transition|GetTransitionDuration)))) (Math|Float|Clamp(Float) (+ (Variables|Transition|GetTransitionProgress) (/ DeltaSeconds (Variables|Transition|GetTransitionDuration))))) (- (Math|Float|MakeLiteralFloat 3.0) (* (Math|Float|MakeLiteralFloat 2.0) (Math|Float|Clamp(Float) (+ (Variables|Transition|GetTransitionProgress) (/ DeltaSeconds (Variables|Transition|GetTransitionDuration))))))) (Math|Float|MakeLiteralFloat 1.0))) :!class /Script/Engine.KismetMaterialLibrary)
  (Rendering|Material|SetScalarParameterValue "/Game/Materials/ParameterCollections/MPC_GlobalWeather.MPC_GlobalWeather" "SnowAmount" (Math|Float|Lerp (Variables|Transition|GetOldSnow) (Variables|WeatherTargets|GetSnowTarget) (select (Variables|Transition|GetIsTransitioning) (* (* (Math|Float|Clamp(Float) (+ (Variables|Transition|GetTransitionProgress) (/ DeltaSeconds (Variables|Transition|GetTransitionDuration)))) (Math|Float|Clamp(Float) (+ (Variables|Transition|GetTransitionProgress) (/ DeltaSeconds (Variables|Transition|GetTransitionDuration))))) (- (Math|Float|MakeLiteralFloat 3.0) (* (Math|Float|MakeLiteralFloat 2.0) (Math|Float|Clamp(Float) (+ (Variables|Transition|GetTransitionProgress) (/ DeltaSeconds (Variables|Transition|GetTransitionDuration))))))) (Math|Float|MakeLiteralFloat 1.0))) :!class /Script/Engine.KismetMaterialLibrary)
  (Rendering|Material|SetScalarParameterValue "/Game/Materials/ParameterCollections/MPC_GlobalWeather.MPC_GlobalWeather" "Temperature" (Math|Float|Lerp (Variables|Transition|GetOldTemperature) (Variables|WeatherTargets|GetTemperatureTargetC) (select (Variables|Transition|GetIsTransitioning) (* (* (Math|Float|Clamp(Float) (+ (Variables|Transition|GetTransitionProgress) (/ DeltaSeconds (Variables|Transition|GetTransitionDuration)))) (Math|Float|Clamp(Float) (+ (Variables|Transition|GetTransitionProgress) (/ DeltaSeconds (Variables|Transition|GetTransitionDuration))))) (- (Math|Float|MakeLiteralFloat 3.0) (* (Math|Float|MakeLiteralFloat 2.0) (Math|Float|Clamp(Float) (+ (Variables|Transition|GetTransitionProgress) (/ DeltaSeconds (Variables|Transition|GetTransitionDuration))))))) (Math|Float|MakeLiteralFloat 1.0))) :!class /Script/Engine.KismetMaterialLibrary)
  (if (Variables|TimeOfDay|GetEnableTimeOfDay)
    (Variables|TimeOfDay|SetTimeOfDayHours (Math|Float|%(Float) (+ (Variables|TimeOfDay|GetTimeOfDayHours) (* (Variables|TimeOfDay|GetTimeSpeedHoursPerSec) DeltaSeconds)) 24.0))
    (Rendering|Material|SetVectorParameterValue "/Game/Materials/ParameterCollections/MPC_GlobalWeather.MPC_GlobalWeather" "SunColor" (Math|Color|Lerp(LinearColor) (select (< (Math|Float|Floor (* (/ (Math|Float|%(Float) (+ (Variables|TimeOfDay|GetTimeOfDayHours) (* (Variables|TimeOfDay|GetTimeSpeedHoursPerSec) DeltaSeconds)) 24.0) (Math|Float|MakeLiteralFloat 24.0)) (Math|Float|MakeLiteralFloat 4.0))) (Math|Float|MakeLiteralFloat 1.0)) (Utilities|Struct|MakeLinearColor 0.05 0.07 0.15 1.0) (select (< (Math|Float|Floor (* (/ (Math|Float|%(Float) (+ (Variables|TimeOfDay|GetTimeOfDayHours) (* (Variables|TimeOfDay|GetTimeSpeedHoursPerSec) DeltaSeconds)) 24.0) (Math|Float|MakeLiteralFloat 24.0)) (Math|Float|MakeLiteralFloat 4.0))) (Math|Float|MakeLiteralFloat 2.0)) (Utilities|Struct|MakeLinearColor 1.0 0.5 0.2 1.0) (select (< (Math|Float|Floor (* (/ (Math|Float|%(Float) (+ (Variables|TimeOfDay|GetTimeOfDayHours) (* (Variables|TimeOfDay|GetTimeSpeedHoursPerSec) DeltaSeconds)) 24.0) (Math|Float|MakeLiteralFloat 24.0)) (Math|Float|MakeLiteralFloat 4.0))) (Math|Float|MakeLiteralFloat 3.0)) (Utilities|Struct|MakeLinearColor 1.0 0.95 0.85 1.0) (Utilities|Struct|MakeLinearColor 1.0 0.4 0.15 1.0)))) (select (< (Math|Float|Floor (* (/ (Math|Float|%(Float) (+ (Variables|TimeOfDay|GetTimeOfDayHours) (* (Variables|TimeOfDay|GetTimeSpeedHoursPerSec) DeltaSeconds)) 24.0) (Math|Float|MakeLiteralFloat 24.0)) (Math|Float|MakeLiteralFloat 4.0))) (Math|Float|MakeLiteralFloat 1.0)) (Utilities|Struct|MakeLinearColor 1.0 0.5 0.2 1.0) (select (< (Math|Float|Floor (* (/ (Math|Float|%(Float) (+ (Variables|TimeOfDay|GetTimeOfDayHours) (* (Variables|TimeOfDay|GetTimeSpeedHoursPerSec) DeltaSeconds)) 24.0) (Math|Float|MakeLiteralFloat 24.0)) (Math|Float|MakeLiteralFloat 4.0))) (Math|Float|MakeLiteralFloat 2.0)) (Utilities|Struct|MakeLinearColor 1.0 0.95 0.85 1.0) (select (< (Math|Float|Floor (* (/ (Math|Float|%(Float) (+ (Variables|TimeOfDay|GetTimeOfDayHours) (* (Variables|TimeOfDay|GetTimeSpeedHoursPerSec) DeltaSeconds)) 24.0) (Math|Float|MakeLiteralFloat 24.0)) (Math|Float|MakeLiteralFloat 4.0))) (Math|Float|MakeLiteralFloat 3.0)) (Utilities|Struct|MakeLinearColor 1.0 0.4 0.15 1.0) (Utilities|Struct|MakeLinearColor 0.05 0.07 0.15 1.0)))) (- (* (/ (Math|Float|%(Float) (+ (Variables|TimeOfDay|GetTimeOfDayHours) (* (Variables|TimeOfDay|GetTimeSpeedHoursPerSec) DeltaSeconds)) 24.0) (Math|Float|MakeLiteralFloat 24.0)) (Math|Float|MakeLiteralFloat 4.0)) (Math|Float|Floor (* (/ (Math|Float|%(Float) (+ (Variables|TimeOfDay|GetTimeOfDayHours) (* (Variables|TimeOfDay|GetTimeSpeedHoursPerSec) DeltaSeconds)) 24.0) (Math|Float|MakeLiteralFloat 24.0)) (Math|Float|MakeLiteralFloat 4.0))))) :!class /Script/Engine.KismetMaterialLibrary)
    (Rendering|Material|SetVectorParameterValue "/Game/Materials/ParameterCollections/MPC_GlobalWeather.MPC_GlobalWeather" "SkyTint" (Math|Color|Lerp(LinearColor) (select (< (Math|Float|Floor (* (/ (Math|Float|%(Float) (+ (Variables|TimeOfDay|GetTimeOfDayHours) (* (Variables|TimeOfDay|GetTimeSpeedHoursPerSec) DeltaSeconds)) 24.0) (Math|Float|MakeLiteralFloat 24.0)) (Math|Float|MakeLiteralFloat 4.0))) (Math|Float|MakeLiteralFloat 1.0)) (Utilities|Struct|MakeLinearColor 0.02 0.03 0.08 1.0) (select (< (Math|Float|Floor (* (/ (Math|Float|%(Float) (+ (Variables|TimeOfDay|GetTimeOfDayHours) (* (Variables|TimeOfDay|GetTimeSpeedHoursPerSec) DeltaSeconds)) 24.0) (Math|Float|MakeLiteralFloat 24.0)) (Math|Float|MakeLiteralFloat 4.0))) (Math|Float|MakeLiteralFloat 2.0)) (Utilities|Struct|MakeLinearColor 0.8 0.5 0.5 1.0) (select (< (Math|Float|Floor (* (/ (Math|Float|%(Float) (+ (Variables|TimeOfDay|GetTimeOfDayHours) (* (Variables|TimeOfDay|GetTimeSpeedHoursPerSec) DeltaSeconds)) 24.0) (Math|Float|MakeLiteralFloat 24.0)) (Math|Float|MakeLiteralFloat 4.0))) (Math|Float|MakeLiteralFloat 3.0)) (Utilities|Struct|MakeLinearColor 0.6 0.75 1.0 1.0) (Utilities|Struct|MakeLinearColor 0.7 0.3 0.3 1.0)))) (select (< (Math|Float|Floor (* (/ (Math|Float|%(Float) (+ (Variables|TimeOfDay|GetTimeOfDayHours) (* (Variables|TimeOfDay|GetTimeSpeedHoursPerSec) DeltaSeconds)) 24.0) (Math|Float|MakeLiteralFloat 24.0)) (Math|Float|MakeLiteralFloat 4.0))) (Math|Float|MakeLiteralFloat 1.0)) (Utilities|Struct|MakeLinearColor 0.8 0.5 0.5 1.0) (select (< (Math|Float|Floor (* (/ (Math|Float|%(Float) (+ (Variables|TimeOfDay|GetTimeOfDayHours) (* (Variables|TimeOfDay|GetTimeSpeedHoursPerSec) DeltaSeconds)) 24.0) (Math|Float|MakeLiteralFloat 24.0)) (Math|Float|MakeLiteralFloat 4.0))) (Math|Float|MakeLiteralFloat 2.0)) (Utilities|Struct|MakeLinearColor 0.6 0.75 1.0 1.0) (select (< (Math|Float|Floor (* (/ (Math|Float|%(Float) (+ (Variables|TimeOfDay|GetTimeOfDayHours) (* (Variables|TimeOfDay|GetTimeSpeedHoursPerSec) DeltaSeconds)) 24.0) (Math|Float|MakeLiteralFloat 24.0)) (Math|Float|MakeLiteralFloat 4.0))) (Math|Float|MakeLiteralFloat 3.0)) (Utilities|Struct|MakeLinearColor 0.7 0.3 0.3 1.0) (Utilities|Struct|MakeLinearColor 0.02 0.03 0.08 1.0)))) (- (* (/ (Math|Float|%(Float) (+ (Variables|TimeOfDay|GetTimeOfDayHours) (* (Variables|TimeOfDay|GetTimeSpeedHoursPerSec) DeltaSeconds)) 24.0) (Math|Float|MakeLiteralFloat 24.0)) (Math|Float|MakeLiteralFloat 4.0)) (Math|Float|Floor (* (/ (Math|Float|%(Float) (+ (Variables|TimeOfDay|GetTimeOfDayHours) (* (Variables|TimeOfDay|GetTimeSpeedHoursPerSec) DeltaSeconds)) 24.0) (Math|Float|MakeLiteralFloat 24.0)) (Math|Float|MakeLiteralFloat 4.0))))) :!class /Script/Engine.KismetMaterialLibrary)))

(fn ConstructionScript)

(fn GetSunColorforHour
  (params (Hour :type Float%20%28double-precision%29)))

(fn GetSkyTintforHour
  (params (Hour :type Float%20%28double-precision%29)))